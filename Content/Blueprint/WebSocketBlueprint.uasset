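; WebSocketBlueprint is an actor that acts as a simple echo handler for a WebSocket server in the level.
; On BeginPlay it takes the first WebSocketServerActor found and binds to its connect and JSON message events.
; Connections print the host; messages print their Type and are sent back unchanged through SendServerJsonMessage.
; A timer-enabled flag (定时器开启) is only set to false and never read here.
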(event Custom|OnConnect_Event
  (params (Host :type String) (Port :type Integer) (Origin :type String))
  (Development|PrintString Host))

(event Custom|OnJsonMessage_Event
  (params (Type :type String) (Command :type String) (brief :type String))
  (Development|PrintString Type)
  (Variables|Default|Set定时器开启 false)
  (Class|WebSocketServerActor|SendServerJsonMessage (Utilities|Array|Get(acopy) (stale EventBeginPlay _outactors)) Type Command brief))

(event EventBeginPlay
  (Variables|Default|Set定时器开启 false)
  (bind _outactors (Actor|GetAllActorsOfClass "/Script/WebSocketServer.WebSocketServerActor"))
  (EventDispatchers|AssignOnJsonMessage (Utilities|Array|Get(acopy) _outactors) (delegate Custom|OnJsonMessage_Event))
  (EventDispatchers|BindEventtoOnConnect (Utilities|Array|Get(acopy) _outactors) (delegate Custom|OnConnect_Event)))

(event Collision|EventActorBeginOverlap
  (params (OtherActor :type Actor%20Object%20Reference)))

(event EventTick
  (params (DeltaSeconds :type Float%20%28single-precision%29)))

(fn ConstructionScript)